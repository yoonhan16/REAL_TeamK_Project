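; BP_ElevatorDoor is a two-panel sliding elevator door that opens and closes through OpenDoor and CloseDoor events.
; Each event plays its own timeline, whose track drives a Lerp of LeftDoor and RightDoor relative Y in opposite directions.
; Closing uses a separate timeline with swapped endpoints rather than reversing the opening one.
; Both events take a Player parameter but do not use it.
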(event Custom|OpenDoor
  (params (Player :type Actor%20Object%20Reference))
  (bind _newtrack_0 (Timeline|Open%20Door%20T Play)
    (:Update
      (Utilities|FlowControl|Sequence
        (:then_0
          (Transformation|SetRelativeLocation (Variables|Default|GetLeftDoor) (Math|Vector|MakeVector 0.0 (Math|Float|Lerp -5e+01 -155.0 _newtrack_0) 0.0) false false))
        (:then_1
          (Transformation|SetRelativeLocation (Variables|Default|GetRightDoor) (Math|Vector|MakeVector 0.0 (Math|Float|Lerp 5e+01 155.0 _newtrack_0) 0.0) false false))))))

(event Custom|CloseDoor
  (params (Player :type Actor%20Object%20Reference))
  (bind _newtrack_0 (Timeline|Timeline Play)
    (:Update
      (Utilities|FlowControl|Sequence
        (:then_0
          (Transformation|SetRelativeLocation (Variables|Default|GetLeftDoor) (Math|Vector|MakeVector 0.0 (Math|Float|Lerp -155.0 -5e+01 _newtrack_0) 0.0) false false))
        (:then_1
          (Transformation|SetRelativeLocation (Variables|Default|GetRightDoor) (Math|Vector|MakeVector 0.0 (Math|Float|Lerp 155.0 5e+01 _newtrack_0) 0.0) false false))))))

(fn ConstructionScript)