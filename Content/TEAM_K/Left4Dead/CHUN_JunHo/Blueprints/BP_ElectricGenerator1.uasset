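; Electric generator Blueprint that, on interaction, restores lighting and triggers a floor collapse.
; Interact prints a debug message, sets DidTask on the player character, then looks up the elevator button and collapsing floor by class.
; Both of the button's light arrays switch on, with timed off/on calls making the first flicker, and the floor's Collapse is called.
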(event EventInteract
  (params (Player :type Character%20Object%20Reference))
  (Development|PrintString "Hello")
  (bind _returnvalue (Actor|GetActorOfClass "/Game/ThirdPerson/Blueprints/BP_ThirdPersonCharacter.BP_ThirdPersonCharacter_C"))
  (Variables|/Game/ThirdPerson/Blueprints/BP_ThirdPersonCharacter.BP_ThirdPersonCharacter_C|SetbDidTask? _returnvalue true)
  (Utilities|FlowControl|Sequence
    (:then_0
      (bind _returnvalue_2 (Actor|GetActorOfClass "/Game/Blueprints/BP_ElevatorButton.BP_ElevatorButton_C"))
      (Utilities|FlowControl|Sequence
        (:then_0
          (for _array_element (Variables|/Game/Blueprints/BP_ElevatorButton.BP_ElevatorButton_C|GetLight1Array _returnvalue_2)
            (Class|BPILightsInterface|Lightson(Message) _array_element)
            (Utilities|Time|SetTimerbyFunctionName _array_element "LightsOff" 0.2)
            (Utilities|Time|SetTimerbyFunctionName _array_element "LightsOn" 0.5 false 0.2)))
        (:then_1
          (for _array_element_2 (Variables|/Game/Blueprints/BP_ElevatorButton.BP_ElevatorButton_C|GetLight2Array _returnvalue_2)
            (Class|BPILightsInterface|Lightson(Message) _array_element_2)))))
    (:then_1
      (bind _returnvalue_3 (Actor|GetActorOfClass "/Game/Blueprints/BP_CollapsingFloor2.BP_CollapsingFloor2_C"))
      (Default|Collapse _returnvalue_3))))

(fn ConstructionScript)