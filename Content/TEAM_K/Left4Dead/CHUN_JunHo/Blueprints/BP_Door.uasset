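; BP_Door is an interactable hinged door that toggles open and closed.
; Interact checks the IsInteracted flag, calls Open or Close, then flips the flag.
; Two separate timelines lerp the door mesh's yaw between closed and 90 degrees, each played from start.
; Collision is disabled while the door swings and restored when the timeline finishes.
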(event Custom|Open
  (bind _door (Variables|Default|GetDoor))
  (bind _newtrack_0 (Timeline|Timeline PlayFromStart)
    (:Update
      (Transformation|SetRelativeRotation _door (Math|Rotator|MakeRotator 0.0 0.0 (Math|Float|Lerp 0.0 9e+01 _newtrack_0)) false false)
      (Collision|SetCollisionEnabled _door "NoCollision"))
    (:Finished
      (Collision|SetCollisionEnabled _door "QueryAndPhysics"))))

(event Custom|Close
  (bind _door (Variables|Default|GetDoor))
  (bind _newtrack_0 (Timeline|Timeline_0 PlayFromStart)
    (:Update
      (Transformation|SetRelativeRotation _door (Math|Rotator|MakeRotator 0.0 0.0 (Math|Float|Lerp 9e+01 0.0 _newtrack_0)) false false)
      (Collision|SetCollisionEnabled _door "NoCollision"))
    (:Finished
      (Collision|SetCollisionEnabled _door "QueryAndPhysics"))))

(event EventInteract
  (params (Player :type Character%20Object%20Reference))
  (if (Variables|Default|GetbIsInteracted?)
    (CallFunction|Close)
    (Variables|Default|SetbIsInteracted? false)
    (else
      (CallFunction|Open)
      (Variables|Default|SetbIsInteracted? true))))

(fn ConstructionScript)