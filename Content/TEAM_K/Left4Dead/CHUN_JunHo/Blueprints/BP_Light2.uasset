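; BP_Light2 is a light actor with events that switch it on and off.
; Both events act only when IsOn is set, changing RectLight visibility and the Light component's LightIntensity material parameter together.
; Lightson also requires the DidTask flag on the BP_ThirdPersonCharacter it finds in the level.
; A toggle that flips IsOn is present but never runs.
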(event EventLightsOff
  (if (Variables|Default|GetbIsOn?)
    (Rendering|SetVisibility (Variables|Default|GetRectLight) false false)
    (Rendering|Material|SetScalarParameterValueonMaterials (Variables|Default|GetLight) "LightIntensity" 0.0)))

(event EventLightson
  (bind _returnvalue (Actor|GetActorOfClass "/Game/ThirdPerson/Blueprints/BP_ThirdPersonCharacter.BP_ThirdPersonCharacter_C"))
  (if (Variables|/Game/ThirdPerson/Blueprints/BP_ThirdPersonCharacter.BP_ThirdPersonCharacter_C|GetbDidTask? _returnvalue)
    (if (Variables|Default|GetbIsOn?)
      (Rendering|SetVisibility (Variables|Default|GetRectLight) true false)
      (Rendering|Material|SetScalarParameterValueonMaterials (Variables|Default|GetLight) "LightIntensity" 1.0))))

(fn ConstructionScript)